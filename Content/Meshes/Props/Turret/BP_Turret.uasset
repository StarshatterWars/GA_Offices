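; Automated turret that detects, tracks and fires on the player while active.
; Each tick, delayed range and Visibility line-trace checks set flags that steer the barrels toward the player with clamped pitch, or back to the start rotation.
; A gate throttles fire, spawning projectiles and muzzle explosions from both barrel sockets after random delays.
; It also calls player spotted or lost events to update the level Blueprint.
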(event Custom|UpdateInRange
  (bind _shootresponsespeed (Variables|Default|GetShootResponseSpeed))
  ;[1 1 1] ChecksIfThePlayerIsInRange
  (if (<= (Transformation|GetDistanceTo self (Game|Player|GetPlayerPawn 0)) (Variables|Default|GetTurretRange))
    (Utilities|FlowControl|Delay _shootresponsespeed)
    (Variables|Default|SetTargetInRange true)
    (else
      (Utilities|FlowControl|Delay _shootresponsespeed)
      (Variables|Default|SetTargetInRange false))))

(event Custom|UpdateBehindCover
  (bind _lostresponsespeed (Variables|Default|GetLostResponseSpeed))
  ;[1 1 1] ChecksIfThePlayerIsBehindCover
  (bind _outhit (Collision|LineTraceByChannel (Transformation|GetWorldLocation (Variables|Default|GetTurretBarrels)) (Transformation|GetActorLocation (Game|Player|GetPlayerPawn 0)) "TraceTypeQuery1" false 0 "None"))
  (if (== (Utilities|GetClass (.HitActor (Collision|BreakHitResult _outhit))) "/Game/Blueprints/MyCharacter.MyCharacter_C")
    (Utilities|FlowControl|Delay _lostresponsespeed)
    (Variables|Default|SetTargetBehindCover false)
    (else
      (Utilities|FlowControl|Delay _lostresponsespeed)
      (Variables|Default|SetTargetBehindCover true))))

(event Custom|FireWeapons
  (bind _turretbarrels (Variables|Default|GetTurretBarrels))
  (bind _turretbarrels_2 (Variables|Default|GetTurretBarrels))
  (bind _returnvalue (Transformation|GetSocketLocation _turretbarrels "RightBarrel"))
  (bind _returnvalue_2 (Transformation|GetSocketRotation _turretbarrels "RightBarrel"))
  (bind _returnvalue_3 (Transformation|GetSocketLocation _turretbarrels_2 "LeftBarrel"))
  (bind _returnvalue_4 (Transformation|GetSocketRotation _turretbarrels_2 "LeftBarrel"))
  (bind _returnvalue_5 (Math|Transform|MakeTransform _returnvalue_3 _returnvalue_4 "0.100000,0.100000,0.100000"))
  (bind _returnvalue_6 (Math|Transform|MakeTransform _returnvalue _returnvalue_2 "0.100000,0.100000,0.100000"))
  ;[1 1 1] SpawnsBlueprintProjectile
  (if (Variables|Default|GetTargetInRange)
    (if (not (Variables|Default|GetTargetBehindCover))
      (Utilities|FlowControl|Gate false :!label _label
        (:Exit
          (Utilities|FlowControl|Sequence
            (:then_0
              (Utilities|FlowControl|Delay (Math|Random|RandomFloatinRange 0.1 0.5))
              (Utilities|FlowControl|Sequence
                (:then_0
                  (Game|SpawnActorfromClass "/Game/Meshes/Props/Turret/Projectile/Gat_BP_Projectile.Gat_BP_Projectile_C" _returnvalue_5 false 0))
                (:then_1
                  (goto _label Open))
                (:then_2
                  (Game|SpawnActorfromClass "/Game/Blueprints/Blueprint_Effect_Explosion.Blueprint_Effect_Explosion_C" _returnvalue_5 false 0))))
            (:then_1
              (goto _label Close))
            (:then_2
              (Utilities|FlowControl|Delay (Math|Random|RandomFloatinRange 0.2 0.5))
              (Utilities|FlowControl|Sequence
                (:then_0
                  (Game|SpawnActorfromClass "/Game/Meshes/Props/Turret/Projectile/Gat_BP_Projectile.Gat_BP_Projectile_C" _returnvalue_6 false 0))
                (:then_1
                  (Game|SpawnActorfromClass "/Game/Blueprints/Blueprint_Effect_Explosion.Blueprint_Effect_Explosion_C" _returnvalue_6 false 0))))))))))

(event Custom|UpdateRot
  (bind _returnvalue (Game|Player|GetPlayerPawn 0))
  (bind _turretbarrels (Variables|Default|GetTurretBarrels))
  (bind _returnvalue_2 (Transformation|GetWorldLocation _turretbarrels))
  (bind _returnvalue_3 (Transformation|GetActorLocation _returnvalue))
  (bind _returnvalue_4 (Math|Rotator|FindLookatRotation _returnvalue_2 _returnvalue_3))
  (bind (_pitch _yaw) (Class|KismetMathLibrary|BreakRot _returnvalue_4))
  ;[1 1 1] UpdatesTheTurretsRotationToFaceThePlayer
  (if (Variables|Default|GetTargetInRange)
    (if (Variables|Default|GetTargetBehindCover)
      ;[1 1 1] Rotates The Turret To The Startup Position When The Player Is Out Of Range Or No Longer Visible
      (Transformation|SetWorldRotation (Variables|Default|GetTurretBarrels) (Math|Interpolation|RInterpTo (Transformation|GetWorldRotation (Variables|Default|GetTurretBarrels)) (Variables|Default|GetStartupPosition) (Variables|Default|GetDeltaSeconds) 2.0) false :!label _label)
      (else
        (Transformation|SetWorldRotation (Variables|Default|GetTurretBarrels) (Math|Interpolation|RInterpTo (Transformation|GetWorldRotation (Variables|Default|GetTurretBarrels)) (Class|KismetMathLibrary|MakeRot (Math|Float|ClampAngle (- _pitch (Variables|Default|GetFireAccuracy)) -65.0 0.0) _yaw 0.0) (Variables|Default|GetDeltaSeconds) (Variables|Default|GetRotationSpeed)) false)))
    (else
      (goto _label))))

(event Custom|UpdateLevelBlueprint
  ;[1 1 1] Update Level Blueprint
  (if (Variables|Default|GetTargetInRange)
    (if (Variables|Default|GetTargetBehindCover)
      (Default|CallPlayerLost :!label _label)
      (else
        (Default|CallPlayerSPotted)))
    (else
      (goto _label))))

(event EventTick
  (params (DeltaSeconds :type Float%20%28single-precision%29))
  ;[1 1 1] DeltaTimeReference
  (Variables|Default|SetDeltaSeconds DeltaSeconds)
  (Utilities|IsValid (Game|Player|GetPlayerPawn 0)
    (:Is%20Valid
      (if (Variables|Default|GetActive)
        (CallFunction|UpdateinRange)
        (CallFunction|UpdateBehindCover)
        (CallFunction|UpdateRot)
        (CallFunction|FireWeapons)
        (CallFunction|UpdateLevelBlueprint)))))

(event EventBeginPlay
  ;[1 1 1] Sets Start Up Position
  (Variables|Default|SetStartupPosition (Transformation|GetWorldRotation (Variables|Default|GetTurretBarrels))))

(fn ConstructionScript)