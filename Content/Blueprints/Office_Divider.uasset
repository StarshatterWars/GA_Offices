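; Office divider hiding spot that hides the player from the Room07 tracking security cameras.
; Overlapping its Box sets the character's Hidden flag, and a 5-second delay then opens a gate on Tick if the player is still inside.
; Tick then finds the cameras and calls PlayerHidden through a DoOnce inside the loop, so only the first one receives it.
; Ending overlap clears Hidden, closes both gates and resets the DoOnce.
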(event OnComponentBeginOverlap(Box)
  (params (OtherActor :type Actor%20Object%20Reference) (OtherComp :type Primitive%20Component%20Object%20Reference) (OtherBodyIndex :type Integer) (bFromSweep :type Boolean) (SweepResult :type Hit%20Result%20Structure%20%28by%20ref%29))
  (if (== (Utilities|GetClass OtherActor) "/Game/Blueprints/MyCharacter.MyCharacter_C")
    (Variables|/Game/Blueprints/MyCharacter.MyCharacter_C|SetHidden (stale EventBeginPlay _asmy_character) true)
    (Utilities|FlowControl|Sequence
      (:then_0
        (goto _label Open))
      (:then_1
        (Utilities|FlowControl|Delay 5.0)
        (Utilities|FlowControl|Gate true :!label _label
          (:Exit
            (Utilities|FlowControl|Gate true) ; enters at Open
          ))))))

(event EventBeginPlay
  (bind _asmy_character (Utilities|Casting|CastToMyCharacter (Game|GetPlayerCharacter 0))))

(event EventActorBeginOverlap
  (params (OtherActor :type Actor%20Object%20Reference)))

(event EventTick
  (params (DeltaSeconds :type Float%20%28single-precision%29))
  (Utilities|FlowControl|Gate true
    (:Exit
      (bind _outactors (Actor|GetAllActorsOfClass "/Game/Assets/Blueprints/BP_Security_Camera_Tracking_Room07.BP_Security_Camera_Tracking_Room07_C"))
      (for _array_element _outactors
        (Utilities|FlowControl|DoOnce false
          (:Completed
            (Default|PlayerHidden _array_element)))))))

(event EventActorEndOverlap
  (params (OtherActor :type Actor%20Object%20Reference))
  (if (== (Utilities|GetClass OtherActor) "/Game/Blueprints/MyCharacter.MyCharacter_C")
    (Variables|/Game/Blueprints/MyCharacter.MyCharacter_C|SetHidden (stale EventBeginPlay _asmy_character) false)
    (Utilities|FlowControl|Sequence
      (:then_0
        (Utilities|FlowControl|Gate true) ; enters at Close
      )
      (:then_1
        (Utilities|FlowControl|DoOnce false) ; enters at Reset
      )
      (:then_2
        (Utilities|FlowControl|Gate true) ; enters at Close
      ))))

(fn ConstructionScript)