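; BP_Safe is an interactable safe that opens when the player presses E inside its trigger box, provided its SafeOpen flag is set.
; Box overlap opens and closes a gate on the key input, and a DoOnce makes the opening run only once.
; Chained timelines spin the handle, then swing the door by lerping their rotations, and finally call the SafeOpen dispatcher.
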(event OnComponentBeginOverlap(Box)
  (params (OtherActor :type Actor%20Object%20Reference) (OtherComp :type Primitive%20Component%20Object%20Reference) (OtherBodyIndex :type Integer) (bFromSweep :type Boolean) (SweepResult :type Hit%20Result%20Structure%20%28by%20ref%29))
  (Utilities|FlowControl|Gate true) ; enters at Open
)

(event OnComponentEndOverlap(Box)
  (params (OtherActor :type Actor%20Object%20Reference) (OtherComp :type Primitive%20Component%20Object%20Reference) (OtherBodyIndex :type Integer))
  (Utilities|FlowControl|Gate true) ; enters at Close
)

(event Input|KeyboardEvents|E
  (:Pressed
    (Utilities|FlowControl|Gate true
      (:Exit
        (if (Variables|Default|GetSafeOpen)
          (Utilities|FlowControl|DoOnce false
            (:Completed
              (bind _handledriver (Timeline|Timeline_0 Play)
                (:Update
                  (Transformation|SetRelativeRotation (Variables|Default|GetHandle) (Math|Rotator|Lerp(Rotator) "0, 0, 0" "520.000000, 0, 0" _handledriver) false))
                (:Finished
                  (bind _doordriver (Timeline|Timeline_1 Play)
                    (:Update
                      (Transformation|SetRelativeRotation (Variables|Default|GetDoor) (Math|Rotator|Lerp(Rotator) "0, 0, 0" "0.000000,-90.000000, 0" _doordriver) false))
                    (:Finished
                      (Default|CallSafeOpen))))))))))))

(fn ConstructionScript)