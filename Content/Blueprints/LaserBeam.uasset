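; LaserBeam is a hazard actor that moves vertically and reports when the player character touches it.
; After a random start delay, a timeline at a randomized play rate drives its Z offset from the starting location, desynchronizing separate instances.
; An overlap on Box1 by MyCharacter calls the PlayerTouched dispatcher through a DoOnce, which the Reset event re-arms.
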(event OnComponentBeginOverlap(Box1)
  (params (OtherActor :type Actor%20Object%20Reference) (OtherComp :type Primitive%20Component%20Object%20Reference) (OtherBodyIndex :type Integer) (bFromSweep :type Boolean) (SweepResult :type Hit%20Result%20Structure%20%28by%20ref%29))
  (if (== (Utilities|GetClass OtherActor) "/Game/Blueprints/MyCharacter.MyCharacter_C")
    (Utilities|FlowControl|DoOnce false
      (:Completed
        (Default|CallPlayerTouched)))))

(event Custom|Reset
  (Utilities|FlowControl|DoOnce false) ; enters at Reset
)

(event EventBeginPlay
  (Variables|Default|SetStartLoc (Transformation|GetActorLocation))
  (Utilities|FlowControl|Delay (Math|Random|RandomFloatinRange 0.5 3.0))
  (Components|Timeline|SetPlayRate (Math|Random|RandomFloatinRange 0.7 1.3))
  (bind _newtrack_0 (Timeline|Timeline_0 Play)
    (:Update
      (Transformation|SetActorLocation (Math|Vector|MakeVector (.X (Math|Vector|BreakVector (Variables|Default|GetStartLoc))) (.Y (Math|Vector|BreakVector (Variables|Default|GetStartLoc))) (+ (.Z (Math|Vector|BreakVector (Variables|Default|GetStartLoc))) (* _newtrack_0 2e+02))) false))))

(fn ConstructionScript)