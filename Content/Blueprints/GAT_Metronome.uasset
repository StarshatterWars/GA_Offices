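; Metronome that broadcasts quarter, eighth and sixteenth beat events, plus half-measure and measure events, from a configurable BPM and beats per measure.
; Activate derives beat intervals, then Tick compares real time to each next-beat timestamp within a one-frame-delta window.
; Eighth and quarter hits feed counters for half-measure and measure events.
; The PushNewValuesOn enum selects which boundary runs PushChanges, re-activating the clock with the current settings.
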(event Custom|Start
  (Default|CallStarted)
  (Components|Activation|Activate))

(event Custom|Stop
  (Variables|Default|SetActive false))

(event Custom|PushChanges
  (Variables|Default|SetInternalBPM (Variables|Default|GetBeatsPerMin))
  (Variables|Default|SetInternalBeatsPerMeasure (Variables|Default|GetBeatsPerMeasure))
  (Components|Activation|Activate))

(event EventTick
  (params (DeltaSeconds :type Float%20%28single-precision%29))
  (if (Variables|Default|GetActive)
    (Variables|Default|SetCurrentDeltaTime DeltaSeconds)
    (Utilities|FlowControl|Sequence
      (:then_0
        (|Check16th
          (:Out
            (|CheckForPushChanges))))
      (:then_1
        (|Check8thBeat
          (:Out
            (|CheckForPushChanges_2
              (:NewParam
                (|CheckHalfMeasure
                  (:Out
                    (|CheckForPushChanges_3))))))))
      (:then_2
        (|Check4thBeat
          (:Out
            (|CheckForPushChanges_4
              (:NewParam
                (|CheckMeasure
                  (:Out
                    (|CheckForPushChanges_5)))))))))))

(fn ConstructionScript)

(fn Check4thBeats01
  (bind _returnvalue (Utilities|Time|GetRealTimeSeconds))
  (bind _currentdeltatime (Variables|Default|GetCurrentDeltaTime))
  (bind _returnvalue_2 (/ _currentdeltatime 1.0))
  (if (and (>= _returnvalue (- (Variables|Default|GetNext4thBeat) _returnvalue_2)) (<= _returnvalue (+ (Variables|Default|GetNext4thBeat) _returnvalue_2)))
    (Default|CallTrigger4thBeat)
    (Variables|Default|SetNext4thBeat (+ (Variables|Default|GetNext4thBeat) (Variables|Default|GetBeat4th))))
  (return))

(fn Check8thBeats01
  (bind _currentdeltatime (Variables|Default|GetCurrentDeltaTime))
  (bind _returnvalue (/ _currentdeltatime 1.0))
  (if (and (>= (Utilities|Time|GetRealTimeSeconds) (- (Variables|Default|GetNext8thBeat) _returnvalue)) (<= (Utilities|Time|GetRealTimeSeconds) (+ (Variables|Default|GetNext8thBeat) _returnvalue)))
    (Default|CallTrigger8thBeat)
    (Variables|Default|SetNext8thBeat (+ (Variables|Default|GetNext8thBeat) (Variables|Default|GetBeat8th))))
  (return))

(fn Check16thBeats01
  (bind _currentdeltatime (Variables|Default|GetCurrentDeltaTime))
  (bind _returnvalue (/ _currentdeltatime 1.0))
  (if (and (>= (Utilities|Time|GetRealTimeSeconds) (- (Variables|Default|GetNext16thBeat) _returnvalue)) (<= (Utilities|Time|GetRealTimeSeconds) (+ (Variables|Default|GetNext16thBeat) _returnvalue)))
    (Default|CallTrigger16thBeat)
    (Variables|Default|SetNext16thBeat (+ (Variables|Default|GetNext16thBeat) (Variables|Default|GetBeat16th))))
  (return))